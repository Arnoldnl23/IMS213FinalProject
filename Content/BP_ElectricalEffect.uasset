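; Timed electrical hazard that penalizes the player's score and teleports them back to spawn on contact with live sparks.
; After a start delay scaled by OffsetAmount, a self-calling event toggles three spark components on and off at fixed intervals.
; The first spark's visibility gates the damage on trigger overlap.
; Tick repeats the check against the last overlapping actor, catching players inside when sparks reappear.
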(event `Toggle Sparks`
  ;[1 1 1] Toggles the psarks to appear and dissappear
  (`KismetSystemLibrary.Delay` 2.0)
  (`SceneComponent.ToggleVisibility` (`self.P_Sparks`) false)
  (`SceneComponent.ToggleVisibility` (`self.P_Sparks2`) false)
  (`SceneComponent.ToggleVisibility` (`self.P_Sparks3`) false)
  (`KismetSystemLibrary.Delay` 2.5)
  (`self.Toggle Sparks`))

(event `self.ReceiveBeginPlay`
  ;[1 1 1] Toggles the psarks to appear and dissappear
  (`KismetSystemLibrary.Delay` (`KismetMathLibrary.Conv_IntToDouble` (* (`self.offsetAmount`) 2)))
  (`self.Toggle Sparks`))

(event `self.Trigger.OnComponentBeginOverlap`
  (params (OverlappedComponent :type "PrimitiveComponent Object Reference") (OtherActor :type "Actor Object Reference") (OtherComp :type "PrimitiveComponent Object Reference") (OtherBodyIndex :type Integer) (bFromSweep :type Boolean) (SweepResult :type "HitResult Structure (by ref)"))
  (if (`SceneComponent.IsVisible` (`self.P_Sparks`))
    (bind _asbp_first_person_character (cast `/Game/FirstPerson/Blueprints/BP_FirstPersonCharacter` OtherActor))
    (set `/Game/FirstPerson/Blueprints/BP_FirstPersonCharacter.playerScore` (- (`/Game/FirstPerson/Blueprints/BP_FirstPersonCharacter.playerScore` _asbp_first_person_character) 1000) _asbp_first_person_character)
    (`self.K2_SetActorLocation` _asbp_first_person_character (`/Game/FirstPerson/Blueprints/BP_FirstPersonCharacter.SpawnLocation` _asbp_first_person_character) false false)))

(event `self.ReceiveTick`
  (params (DeltaSeconds :type "Float (single-precision)"))
  (if (and (`PrimitiveComponent.IsOverlappingActor` (`self.Trigger`) (stale `self.Trigger.OnComponentBeginOverlap` OtherActor)) (`SceneComponent.IsVisible` (`self.P_Sparks`)))
    (bind _asbp_first_person_character (cast `/Game/FirstPerson/Blueprints/BP_FirstPersonCharacter` (stale `self.Trigger.OnComponentBeginOverlap` OtherActor)))
    (set `/Game/FirstPerson/Blueprints/BP_FirstPersonCharacter.playerScore` (- (`/Game/FirstPerson/Blueprints/BP_FirstPersonCharacter.playerScore` _asbp_first_person_character) 1000) _asbp_first_person_character)
    (`self.K2_SetActorLocation` _asbp_first_person_character (`/Game/FirstPerson/Blueprints/BP_FirstPersonCharacter.SpawnLocation` _asbp_first_person_character) false false)))

(fn `UserConstructionScript`)