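; BP_ResetButton plays back the correct order for a button puzzle by lighting linked buttons one at a time.
; ShowOrder picks one of two fixed sequences, a three-button set or a four-button set, based on IsSet2.
; It clears all seven buttons through TurnAllOff, turns each on with timed delays, then clears them again after a short hold.
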(event `showOrder`
  (params (isSet2 :type Boolean))
  (if isSet2
    (`self.turnAllOff`)
    (`KismetSystemLibrary.Delay` 0.5)
    (`/Game/ImportedModels/BP_SelectButton.buttonOn` (`self.button4`))
    (`KismetSystemLibrary.Delay` 0.5)
    (`/Game/ImportedModels/BP_SelectButton.buttonOn` (`self.button7`))
    (`KismetSystemLibrary.Delay` 0.5)
    (`/Game/ImportedModels/BP_SelectButton.buttonOn` (`self.button5`))
    (`KismetSystemLibrary.Delay` 0.5)
    (`/Game/ImportedModels/BP_SelectButton.buttonOn` (`self.button6`))
    (`KismetSystemLibrary.Delay` 1.0)
    (`self.turnAllOff`)
    (else
      (`self.turnAllOff`)
      (`KismetSystemLibrary.Delay` 0.5)
      (`/Game/ImportedModels/BP_SelectButton.buttonOn` (`self.button1`))
      (`KismetSystemLibrary.Delay` 0.5)
      (`/Game/ImportedModels/BP_SelectButton.buttonOn` (`self.button3`))
      (`KismetSystemLibrary.Delay` 0.5)
      (`/Game/ImportedModels/BP_SelectButton.buttonOn` (`self.button2`))
      (`KismetSystemLibrary.Delay` 1.0)
      (`self.turnAllOff`))))

(event `turnAllOff`
  (for _array_element (`|MakeArray` (`self.button1`) (`self.button3`) (`self.button2`) (`self.button4`) (`self.button5`) (`self.button6`) (`self.button7`))
    (`/Game/ImportedModels/BP_SelectButton.buttonOff` _array_element)))

(fn `UserConstructionScript`)