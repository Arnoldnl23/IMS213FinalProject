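; BP_Door is a gate that opens once the player has collected five keys.
; Each CollectItem call increments a key counter, and reaching five triggers OpenDoor through a DoOnce.
; OpenDoor plays a timeline whose DoorHeight track offsets the gate mesh vertically from the world position cached at BeginPlay.
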(event `Open Door`
  (bind (_direction _door_height) (`Timeline|Open Door Anim`)
    (:`Update`
      (`SceneComponent.K2_SetWorldLocation` (`self.Gate01PreviewMeshOpen`) (`KismetMathLibrary.MakeVector` (`self.startX`) (`self.startY`) (+ _door_height (`self.StartZ`))) false false))))

(event `Collect Item`
  (`/Engine/EditorBlueprintResources/StandardMacros.IncrementInt` (`self.KeysCollected`)
    (:`  `
      (if (== (`self.KeysCollected`) 5)
        (`/Engine/EditorBlueprintResources/StandardMacros.DoOnce` false
          (:`Completed`
            (`self.Open Door`)))))))

(event `self.ReceiveBeginPlay`
  (bind (_returnvalue_x _returnvalue_y _returnvalue_z) (`KismetMathLibrary.BreakVector` (`SceneComponent.K2_GetComponentLocation` (`self.Gate01PreviewMeshOpen`))))
  (set `self.startX` _returnvalue_x)
  (set `self.startY` _returnvalue_y)
  (set `self.StartZ` _returnvalue_z))

(fn `UserConstructionScript`)